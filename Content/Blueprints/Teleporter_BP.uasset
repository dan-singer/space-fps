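; Teleporter actor that starts a teleport when a Character enters its box trigger and ends it when a Character leaves.
; The box overlap events cast to Character and call Teleport or EndTeleport, whose logic is not defined in this Blueprint.
; SetActive toggles the actor's visibility, collision and tick together, and activates the particle system when switched on.
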(event `self.Box.OnComponentBeginOverlap`
  (params (OverlappedComponent :type "PrimitiveComponent Object Reference") (OtherActor :type "Actor Object Reference") (OtherComp :type "PrimitiveComponent Object Reference") (OtherBodyIndex :type Integer) (bFromSweep :type Boolean) (SweepResult :type "HitResult Structure (by ref)"))
  (bind _ascharacter (cast `Character` OtherActor))
  (`self.Teleport` _ascharacter))

(event `self.Box.OnComponentEndOverlap`
  (params (OverlappedComponent :type "PrimitiveComponent Object Reference") (OtherActor :type "Actor Object Reference") (OtherComp :type "PrimitiveComponent Object Reference") (OtherBodyIndex :type Integer))
  (cast `Character` OtherActor)
  (`self.EndTeleport`))

(fn `SetActive`
  (params (Active :type Boolean))
  (`self.SetActorHiddenInGame` (not Active))
  (`self.SetActorEnableCollision` Active)
  (`self.SetActorTickEnabled` Active)
  (if Active
    (`ActorComponent.Activate` (`self.ParticleSystem`) false)))

(fn `UserConstructionScript`)