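; BrokenConsole is an interactable broken console actor that gives off sparks when the player uses it.
; Box overlap begin and end enable and disable input from player controller 0, without checking which actor overlaps.
; Pressing Interact spawns a Sparks actor at the SpawnLoc component's location, then destroys it after a short delay.
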(event `self.Box.OnComponentBeginOverlap`
  (params (OverlappedComponent :type "PrimitiveComponent Object Reference") (OtherActor :type "Actor Object Reference") (OtherComp :type "PrimitiveComponent Object Reference") (OtherBodyIndex :type Integer) (bFromSweep :type Boolean) (SweepResult :type "HitResult Structure (by ref)"))
  (`self.EnableInput` (`GameplayStatics.GetPlayerController` 0)))

(event `self.Box.OnComponentEndOverlap`
  (params (OverlappedComponent :type "PrimitiveComponent Object Reference") (OtherActor :type "Actor Object Reference") (OtherComp :type "PrimitiveComponent Object Reference") (OtherBodyIndex :type Integer))
  (`self.DisableInput` (`GameplayStatics.GetPlayerController` 0)))

(event `InputAction|Interact`
  (params (Key :type "Key Structure"))
  (:`Pressed`
    (bind _returnvalue (`|SpawnActorFromClass` (`self.Sparks`) (`KismetMathLibrary.MakeTransform` (`SceneComponent.K2_GetComponentLocation` (`self.SpawnLoc`))) "Undefined" "OverrideRootScale" null null))
    (`KismetSystemLibrary.Delay` 1.0)
    (`self.K2_DestroyActor` _returnvalue)))

(fn `UserConstructionScript`)