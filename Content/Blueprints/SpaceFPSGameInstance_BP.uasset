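; Game instance Blueprint for a space FPS, providing a function that applies graphics settings through console commands.
; SetGraphicsSettings takes view distance, anti-aliasing, post-process, shadow, texture, effects, foliage and screen percentage values, running one r.* command for each.
; Each command is built by appending the value to the variable name with an empty prefix, leaving no space between name and value.
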(fn `SetGraphicsSettings`
  (params (ViewDistance :type "Float (double-precision)") (AA :type Integer) (PostProcessQuality :type Integer) (ShadowQuality :type Integer) (TextureQuality :type Integer) (EffectsQuality :type Integer) (FoilageQuality :type Integer) (ScreenPercentage :type Integer))
  (`KismetSystemLibrary.ExecuteConsoleCommand` (`KismetStringLibrary.BuildString_Double` "r.ViewDistanceScale" " " ViewDistance) null)
  (`KismetSystemLibrary.ExecuteConsoleCommand` (`KismetStringLibrary.BuildString_Int` "r.PostProcessAAQuality" " " AA) null)
  (`KismetSystemLibrary.ExecuteConsoleCommand` (`KismetStringLibrary.BuildString_Int` "r.PostProcessQuality" " " PostProcessQuality) null)
  (`KismetSystemLibrary.ExecuteConsoleCommand` (`KismetStringLibrary.BuildString_Int` "r.ShadowQuality" " " ShadowQuality) null)
  (`KismetSystemLibrary.ExecuteConsoleCommand` (`KismetStringLibrary.BuildString_Int` "r.TextureQuality" " " TextureQuality) null)
  (`KismetSystemLibrary.ExecuteConsoleCommand` (`KismetStringLibrary.BuildString_Int` "r.EffectsQuality" " " EffectsQuality) null)
  (`KismetSystemLibrary.ExecuteConsoleCommand` (`KismetStringLibrary.BuildString_Int` "r.FoliageQuality" " " FoilageQuality) null)
  (`KismetSystemLibrary.ExecuteConsoleCommand` (`KismetStringLibrary.BuildString_Int` "r.ScreenPercentage" " " ScreenPercentage) null))