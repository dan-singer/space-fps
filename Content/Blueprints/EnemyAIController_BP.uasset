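; Enemy AI controller that runs the Enemy_BT behavior tree on BeginPlay.
; Perception updates for the FirstPersonCharacter write whether it is currently sensed to the CanSeePlayer blackboard key.
; Each Tick copies the IsFiring blackboard key into a controller variable of the same name.
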(event `self.ReceiveBeginPlay`
  (`self.RunBehaviorTree` "/Game/Blueprints/AI/Enemy_BT.Enemy_BT"))

(event `self.AIPerception.OnTargetPerceptionUpdated`
  (params (Actor :type "Actor Object Reference") (Stimulus :type "AIStimulus Structure"))
  (cast `/Game/FirstPersonCPP/Blueprints/FirstPersonCharacter` Actor)
  (`BlackboardComponent.SetValueAsBool` (`AIBlueprintHelperLibrary.GetBlackboard` null) "CanSeePlayer" Stimulus_bSuccessfullySensed))

(event `self.ReceiveTick`
  (params (DeltaSeconds :type "Float (single-precision)"))
  (set `self.IsFiring` (`BlackboardComponent.GetValueAsBool` (`AIBlueprintHelperLibrary.GetBlackboard` null) "IsFiring")))

(fn `UserConstructionScript`)